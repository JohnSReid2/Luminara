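; Fog actor that builds a layered fog effect from stacked mesh planes when play begins.
; It adds static mesh components at evenly spaced Z offsets, with the step set by LayerHeight divided by Resolution.
; The base plane and each added layer get a dynamic material instance, fed the base plane's world Z as MinFrom and LayerHeight as MaxFrom.
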(event `self.ReceiveBeginPlay`
  (bind _plane (`self.Plane`))
  (bind (_returnvalue_x _returnvalue_y _returnvalue_z) (`KismetMathLibrary.BreakVector` (`SceneComponent.K2_GetComponentLocation` _plane)))
  (bind _returnvalue (+ (`self.PreviousLayerH`) (/ (`self.LayerHeight`) (`self.Resolution`))))
  (bind _returnvalue_2 (`PrimitiveComponent.CreateDynamicMaterialInstance` _plane 0 (`PrimitiveComponent.GetMaterial` _plane 0) "None"))
  (set `self.seedheight` _returnvalue_z)
  (`MaterialInstanceDynamic.SetScalarParameterValue` _returnvalue_2 "MinFrom" _returnvalue_z)
  (`MaterialInstanceDynamic.SetScalarParameterValue` _returnvalue_2 "MaxFrom" (`self.LayerHeight`))
  (for _ (range (+ (`self.Resolution`) 1))
    (bind _returnvalue_3 (`AddComponent|NODE_AddStaticMeshComponent-0` :`RelativeTransform` (`KismetMathLibrary.MakeTransform` (`KismetMathLibrary.MakeVector` 0.0 0.0 _returnvalue))))
    (set `self.PreviousLayerH` _returnvalue)
    (bind _returnvalue_4 (`PrimitiveComponent.CreateDynamicMaterialInstance` _returnvalue_3 0 (`PrimitiveComponent.GetMaterial` _returnvalue_3 0) "None"))
    (`MaterialInstanceDynamic.SetScalarParameterValue` _returnvalue_4 "MinFrom" (`self.seedheight`))
    (`MaterialInstanceDynamic.SetScalarParameterValue` _returnvalue_4 "MaxFrom" (`self.LayerHeight`))))

(fn `UserConstructionScript`)